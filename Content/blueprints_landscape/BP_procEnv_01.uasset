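; Procedural environment Blueprint that builds a flat grid mesh with collision on BeginPlay using a ProceduralMesh component.
; CreatingVertices fills a grid of vertices and UVs from XWidth, YLength, MeshScale and UVScale, drawing a long-lived debug sphere at each point.
; CreatingTriangles currently adds only the first triangle, so the created section renders one face of the grid before Material is applied.
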(event EventBeginPlay
  (CallFunction|CreatingVertices)
  (CallFunction|CreatingTriangles)
  (Class|ProceduralMeshComponent|CreateMeshSectionLinearColor (Variables|Default|GetProceduralMesh) 0 (Variables|Default|GetVertices) (Variables|Default|GetTriangles) 0 (Variables|Default|GetUV0) 0 0 0 0 0 true false)
  (Rendering|Material|SetMaterial (Variables|Default|GetProceduralMesh) 0 (Variables|Default|GetMaterial)))

(fn ConstructionScript)

(fn CreatingVertices
  (for _index (range 0 (Variables|Default|GetX_Width))
    (LocalVariables|SetX _index)
    (for _index_2 (range 0 (Variables|Default|GetY_Length))
      (LocalVariables|SetY _index_2)
      (Utilities|Array|Add (Variables|Default|GetVertices) (Math|Vector|MakeVector (* (LocalVariables|GetX) (Variables|Default|GetMeshScale)) (* (LocalVariables|GetY) (Variables|Default|GetMeshScale)) 0.0))
      (Utilities|Array|Add (Variables|Default|GetUV0) (Math|Vector2D|MakeVector2D (* (LocalVariables|GetX) (Variables|Default|GetUVScale)) (* (LocalVariables|GetY) (Variables|Default|GetUVScale))))
      (Rendering|Debug|DrawDebugSphere (Math|Vector|MakeVector (* (LocalVariables|GetX) (Variables|Default|GetMeshScale)) (* (LocalVariables|GetY) (Variables|Default|GetMeshScale)) 0.0) 1e+01 12 "(R=1.000000,G=0.000000,B=0.038562,A=1.000000)" 2e+06 1.0))))

(fn CreatingTriangles
  (Utilities|Array|Add (Variables|Default|GetTriangles) 0)
  (Utilities|Array|Add (Variables|Default|GetTriangles) 1)
  (Utilities|Array|Add (Variables|Default|GetTriangles) (+ (Variables|Default|GetY_Length) 1)))