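; AI villager that alternates between sleeping at the nearest keeper house and working at the hall bar.
; BeginPlay caches bed, bar and table locations from the house and hall actors.
; Self-calling events with delays drive movement, bar-to-random-table trips and status text, switching on the Day_night_cycle clock and a bar overlap check.
; Tick yaws the status display toward the player camera; a leftover farmer timeline is never run.
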(event Custom|at%20work
  (bind _table_02_location (Variables|Default|Gettable_02_location))
  (bind _table_01_location (Variables|Default|Gettable_01_location))
  (bind _table_03_location (Variables|Default|Gettable_03_location))
  (bind _array (Utilities|Array|MakeArray _table_01_location _table_02_location _table_03_location))
  (bind _outitem (Utilities|Array|Random _array))
  (Rendering|Components|TextRender|SetText (Variables|Default|Getstatus_OBJECTIVE) (Utilities|Text|ToText(String) (Variables|Default|Getworking_text)))
  (Utilities|FlowControl|Delay 3.0)
  (Development|PrintText (Utilities|Text|ToText(String) _outitem) true true "(R=1.000000,G=0.019096,B=0.000000,A=1.000000)" 5.0)
  (AI|Navigation|SimpleMovetoLocation (AI|GetAIController self) _outitem)
  (Utilities|FlowControl|Delay 1.0)
  (AI|Navigation|SimpleMovetoLocation (AI|GetAIController self) (Variables|Default|Getmy_work))
  (Utilities|FlowControl|Delay 1.0)
  (CallFunction|CheckTime)
  (if (<= (Variables|Default|Getclocktime_var) 1e+01)
    (CallFunction|AtWork)
    (else
      (CallFunction|GotoBed))))

(event Custom|find%20my%20stuff
  (bind _outactors (Actor|GetAllActorsOfClass "/Game/blueprints_buildings/BP_keeper_house_01.BP_keeper_house_01_C"))
  (bind _asbp_keeper_house_01 (Utilities|Casting|CastToBP_keeper_house_01 (.ReturnValue (Actor|FindNearestActor (Transformation|GetWorldLocation (Variables|Collision|GetCapsuleComponent)) _outactors))))
  (Variables|Default|Setmy%20bed (Variables|/Game/blueprints_buildings/BP_keeper_house_01.BP_keeper_house_01_C|Getlocation_BED_var _asbp_keeper_house_01))
  (Variables|Default|Setmy%20light (Variables|/Game/blueprints_buildings/BP_keeper_house_01.BP_keeper_house_01_C|Getlocation_LIGHT_var _asbp_keeper_house_01))
  (Variables|Default|Setmy%20home (Variables|/Game/blueprints_buildings/BP_keeper_house_01.BP_keeper_house_01_C|Getlocation_HOME_var _asbp_keeper_house_01))
  (bind _returnvalue (Actor|GetActorOfClass "/Game/blueprints_buildings/BP_hall_01.BP_hall_01_C"))
  (bind _asbp_hall_01 (Utilities|Casting|CastToBP_hall_01 _returnvalue))
  (Variables|Default|Settable_01_location (Transformation|GetWorldLocation (Variables|/Game/blueprints_buildings/BP_hall_01.BP_hall_01_C|Gettable__01_location _asbp_hall_01)))
  (Variables|Default|Settable_02_location (Transformation|GetWorldLocation (Variables|/Game/blueprints_buildings/BP_hall_01.BP_hall_01_C|Gettable__02_location _asbp_hall_01)))
  (Variables|Default|Settable_03_location (Transformation|GetWorldLocation (Variables|/Game/blueprints_buildings/BP_hall_01.BP_hall_01_C|Gettable__03_location _asbp_hall_01))))

(event Custom|check%20time
  (bind _returnvalue (Actor|GetActorOfClass "/Game/blueprints_world_mechanics/day_night_cycle.day_night_cycle_C"))
  (bind _asday_night_cycle (Utilities|Casting|CastToday_night_cycle _returnvalue))
  (Variables|Default|Setclocktime_var (Variables|/Game/blueprints_world_mechanics/day_night_cycle.day_night_cycle_C|GetclockTime _asday_night_cycle))
  (Utilities|FlowControl|Delay 1.0))

(event Custom|find%20locations
  (bind _returnvalue (Actor|GetActorOfClass "/Game/blueprints_buildings/BP_hall_01.BP_hall_01_C"))
  (bind _asbp_hall_01 (Utilities|Casting|CastToBP_hall_01 _returnvalue))
  (Variables|Default|Setmy_work (Variables|/Game/blueprints_buildings/BP_hall_01.BP_hall_01_C|Getbar_location_location _asbp_hall_01))
  (Development|PrintText (Utilities|Text|ToText(String) (Variables|/Game/blueprints_buildings/BP_hall_01.BP_hall_01_C|Getbar_location_location _asbp_hall_01))))

(event Custom|go%20to%20work
  (Rendering|Components|TextRender|SetText (Variables|Default|Getstatus_OBJECTIVE) (Utilities|Text|ToText(String) (Variables|Default|Getgotowork_text)))
  (AI|Navigation|SimpleMovetoLocation (AI|GetAIController self) (Variables|Default|Getmy_work))
  (if (Class|PrimitiveComponent|IsOverlappingComponent (Variables|Default|GetSphere) (Variables|/Game/blueprints_buildings/BP_hall_01.BP_hall_01_C|Getbar_collider (stale Custom|find%20my%20stuff _asbp_hall_01)))
    (CallFunction|AtWork)))

(event Custom|go%20to%20bed
  (AI|Navigation|SimpleMovetoLocation (AI|GetAIController self) (Variables|Default|Getmy%20bed))
  (Utilities|FlowControl|Delay 1.0)
  (Rendering|Components|TextRender|SetText (Variables|Default|Getstatus_OBJECTIVE) (Utilities|Text|ToText(String) (Variables|Default|Getsleeping_text)))
  (CallFunction|CheckTime)
  (if (> (Variables|Default|Getclocktime_var) 1.6e+02)
    (CallFunction|GotoWork)
    (else
      (CallFunction|GotoBed))))

(event EventTick
  (params (DeltaSeconds :type Float%20%28single-precision%29))
  (Transformation|SetWorldRotation (Variables|Default|Getstatus_root) (Math|Rotator|MakeRotator 0.0 0.0 (.yaw (Math|Rotator|FindLookatRotation (Transformation|GetWorldLocation (Variables|Collision|GetCapsuleComponent)) (Transformation|GetWorldLocation (Variables|/Script/Engine.Actor|GetRootComponent (Game|GetPlayerCameraManager 0)))))) false false))

(event EventBeginPlay
  (Utilities|FlowControl|Delay 2.0)
  (CallFunction|FindMyStuff)
  (CallFunction|FindLocations)
  (CallFunction|GotoBed))

(fn ConstructionScript)