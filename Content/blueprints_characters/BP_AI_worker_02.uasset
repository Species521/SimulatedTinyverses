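; AI worker character that runs a clock-driven daily routine between bed, marketplace, farm and hall.
; On BeginPlay it caches the nearest BP_worker_house_02 bed plus market and farm locations, then starts at bed.
; Self-calling events poll Day_night_cycle's ClockTime, chaining delayed SimpleMoveTo calls with random detours and hall tables.
; Work and sleep update a status text, whose root yaws toward the camera each Tick.
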(event Custom|go%20to%20hall
  (bind _returnvalue (Actor|GetActorOfClass "/Game/blueprints_buildings/BP_hall_01.BP_hall_01_C"))
  (bind _asbp_hall_01 (Utilities|Casting|CastToBP_hall_01 _returnvalue))
  (bind _output_get (Variables|Default|Sethall_01_location (Transformation|GetWorldLocation (.OutItem (Utilities|Array|Random (Utilities|Array|MakeArray (Variables|/Game/blueprints_buildings/BP_hall_01.BP_hall_01_C|Gettable__01_location _asbp_hall_01) (Variables|/Game/blueprints_buildings/BP_hall_01.BP_hall_01_C|Gettable__02_location _asbp_hall_01) (Variables|/Game/blueprints_buildings/BP_hall_01.BP_hall_01_C|Gettable__03_location _asbp_hall_01)))))))
  (AI|Navigation|SimpleMovetoLocation (AI|GetAIController self) (Variables|Default|Gethall_01_location))
  (Development|PrintText (Utilities|Text|ToText(String) _output_get) true true "(R=0.000000,G=1.000000,B=0.218530,A=1.000000)" 5.0)
  (Utilities|FlowControl|Delay 6.0)
  (if (>= (Variables|Default|Getclocktime_var) 2.8e+02)
    (CallFunction|GotoBed)
    (else
      (CallFunction|GotoWork))))

(event Custom|find%20my%20stuff
  (bind _outactors (Actor|GetAllActorsOfClass "/Game/blueprints_buildings/BP_worker_house_02.BP_worker_house_02_C"))
  (bind _asbp_worker_house_02 (Utilities|Casting|CastToBP_worker_house_02 (.ReturnValue (Actor|FindNearestActor (Transformation|GetWorldLocation (Variables|Collision|GetCapsuleComponent)) _outactors))))
  (Variables|Default|Setmy%20bed (Variables|/Game/blueprints_buildings/BP_worker_house_02.BP_worker_house_02_C|Getlocation_BED_var _asbp_worker_house_02))
  (Variables|Default|Setmy%20light (Variables|/Game/blueprints_buildings/BP_worker_house_02.BP_worker_house_02_C|Getlocation_LIGHT_var _asbp_worker_house_02))
  (Variables|Default|Setmy%20home (Variables|/Game/blueprints_buildings/BP_worker_house_02.BP_worker_house_02_C|Getlocation_HOME_var _asbp_worker_house_02)))

(event Custom|check%20time
  (bind _returnvalue (Actor|GetActorOfClass "/Game/blueprints_world_mechanics/day_night_cycle.day_night_cycle_C"))
  (bind _asday_night_cycle (Utilities|Casting|CastToday_night_cycle _returnvalue))
  (Variables|Default|Setclocktime_var (Variables|/Game/blueprints_world_mechanics/day_night_cycle.day_night_cycle_C|GetclockTime _asday_night_cycle))
  (Utilities|FlowControl|Delay 1.0))

(event Custom|find%20locations
  (bind _returnvalue (Actor|GetActorOfClass "/Game/blueprints_buildings/BP_marketplace_01.BP_marketplace_01_C"))
  (bind _asbp_marketplace_01 (Utilities|Casting|CastToBP_marketplace_01 _returnvalue))
  (Variables|Default|Setmarketplace_01_location (Transformation|GetWorldLocation (Variables|/Game/blueprints_buildings/BP_marketplace_01.BP_marketplace_01_C|Getmarketplce_locator _asbp_marketplace_01)))
  (bind _returnvalue_2 (Actor|GetActorOfClass "/Game/blueprints_buildings/BP_farm_01.BP_farm_01_C"))
  (bind _asbp_farm_01 (Utilities|Casting|CastToBP_farm_01 _returnvalue_2))
  (Variables|Default|Setfarm_01_location (Transformation|GetWorldLocation (Variables|/Game/blueprints_buildings/BP_farm_01.BP_farm_01_C|Getfarm_storage_locator _asbp_farm_01))))

(event Custom|go%20to%20work
  (CallFunction|CheckTime)
  (if (>= (Variables|Default|Getclocktime_var) 2.8e+02)
    (CallFunction|GotoBed)
    (else
      (Rendering|Components|TextRender|SetText (Variables|Default|Getstatus_OBJECTIVE) (Utilities|Text|ToText(String) (Variables|Default|Getworking_text)))
      (bind _randomlocation (Class|NavigationSystemV1|GetRandomLocationinNavigableRadius (Variables|Default|Getmarketplace_01_location) 1e+02 0 0))
      (CallFunction|CheckTime)
      (if (< (Variables|Default|Getclocktime_var) 2.7e+02)
        (AI|Navigation|SimpleMovetoLocation (AI|GetAIController self) _randomlocation)
        (Utilities|FlowControl|Delay 2.0)
        (if (Math|Random|RandomBoolwithWeight 0.5)
          (AI|Navigation|SimpleMovetoLocation (AI|GetAIController self) (Variables|Default|Getfarm_01_location))
          (Utilities|FlowControl|Delay 4.0)
          (if (Math|Random|RandomBool)
            (CallFunction|GotoHall :!label _label)
            (Utilities|FlowControl|Delay 6.0)
            (else
              (bind _randomlocation_2 (Class|NavigationSystemV1|GetRandomLocationinNavigableRadius (Variables|Default|Getmarketplace_01_location) 1e+02 0 0))
              (AI|Navigation|SimpleMovetoLocation (AI|GetAIController self) _randomlocation_2)
              (Utilities|FlowControl|Delay 3.0)))
          (else
            (goto _label)))
        (CallFunction|CheckTime)
        (if (>= (Variables|Default|Getclocktime_var) 2.7e+02)
          (Utilities|FlowControl|Delay (Math|Random|RandomFloatinRange 0.0 1.0))
          (CallFunction|GotoBed)
          (else
            (CallFunction|GotoWork)))
        (else
          (CallFunction|GotoBed))))))

(event Custom|go%20to%20bed
  (bind _my_bed (Variables|Default|Getmy%20bed))
  (AI|Navigation|SimpleMovetoLocation (AI|GetAIController self) _my_bed)
  (Development|PrintText (Utilities|Text|ToText(String) _my_bed) true true "(R=0.994792,G=1.000000,B=0.989583,A=1.000000)" 52.0)
  (Utilities|FlowControl|Delay 1e+01)
  (Rendering|Components|TextRender|SetText (Variables|Default|Getstatus_OBJECTIVE) (Utilities|Text|ToText(String) (Variables|Default|Getsleeping_text)))
  (CallFunction|CheckTime)
  (if (> (Variables|Default|Getclocktime_var) 1.7e+02)
    (Utilities|FlowControl|Delay (Math|Random|RandomFloatinRange 0.0 3.0))
    (CallFunction|GotoWork)
    (else
      (CallFunction|GotoBed))))

(event EventTick
  (params (DeltaSeconds :type Float%20%28single-precision%29))
  (Transformation|SetWorldRotation (Variables|Default|Getstatus_root) (Math|Rotator|MakeRotator 0.0 0.0 (.yaw (Math|Rotator|FindLookatRotation (Transformation|GetWorldLocation (Variables|Collision|GetCapsuleComponent)) (Transformation|GetWorldLocation (Variables|/Script/Engine.Actor|GetRootComponent (Game|GetPlayerCameraManager 0)))))) false false))

(event EventBeginPlay
  (Utilities|FlowControl|Delay 2.0)
  (CallFunction|FindMyStuff)
  (CallFunction|FindLocations)
  (CallFunction|GotoBed))

(fn ConstructionScript)