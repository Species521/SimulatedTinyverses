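; Farmer NPC that follows a daily routine of sleeping at home, working the field and visiting the hall.
; On BeginPlay it caches its nearest house and the farm's field, then picks an activity from the day/night cycle's clock.
; Delay-driven, self-repeating events poll the clock and issue simple move orders, with random field points, hall seats and hall-or-bed choice.
; A status text shows the current objective and yaws toward the camera each tick; unused movement logic remains disconnected.
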(event Custom|decisions_by_time
  (if (< (Variables|Default|Getclocktime_var) 1.6e+02)
    (CallFunction|GotoBed)
    (elif (< (Variables|Default|Getclocktime_var) 2.6e+02)
      (CallFunction|GotoWork)
      (else
        (CallFunction|GotoHall)))))

(event Custom|find%20my%20stuff
  (bind _outactors (Actor|GetAllActorsOfClass "/Game/blueprints_buildings/BP_farmer_house_01.BP_farmer_house_01_C"))
  (bind _asbp_farmer_house_01 (Utilities|Casting|CastToBP_farmer_house_01 (.ReturnValue (Actor|FindNearestActor (Transformation|GetWorldLocation (Variables|Collision|GetCapsuleComponent)) _outactors))))
  (Variables|Default|Setmy%20bed (Variables|/Game/blueprints_buildings/BP_farmer_house_01.BP_farmer_house_01_C|Getlocation_BED_var _asbp_farmer_house_01))
  (Variables|Default|Setmy%20light (Variables|/Game/blueprints_buildings/BP_farmer_house_01.BP_farmer_house_01_C|Getlocation_LIGHT_var _asbp_farmer_house_01))
  (Variables|Default|Setmy%20home (Variables|/Game/blueprints_buildings/BP_farmer_house_01.BP_farmer_house_01_C|Getlocation_HOME_var _asbp_farmer_house_01)))

(event Custom|check%20time
  (bind _returnvalue (Actor|GetActorOfClass "/Game/blueprints_world_mechanics/day_night_cycle.day_night_cycle_C"))
  (bind _asday_night_cycle (Utilities|Casting|CastToday_night_cycle _returnvalue))
  (Variables|Default|Setclocktime_var (Variables|/Game/blueprints_world_mechanics/day_night_cycle.day_night_cycle_C|GetclockTime _asday_night_cycle))
  (Utilities|FlowControl|Delay 0.1))

(event Custom|find%20locations
  (bind _returnvalue (Actor|GetActorOfClass "/Game/blueprints_buildings/BP_farm_01.BP_farm_01_C"))
  (bind _asbp_farm_01 (Utilities|Casting|CastToBP_farm_01 _returnvalue))
  (Variables|Default|SetField%20Location (Variables|/Game/blueprints_buildings/BP_farm_01.BP_farm_01_C|Getfield_location _asbp_farm_01))
  (Variables|Default|Setmy_work (Variables|/Game/blueprints_buildings/BP_farm_01.BP_farm_01_C|Getfield_location_location _asbp_farm_01))
  (Development|PrintText (Utilities|Text|ToText(String) (Variables|/Game/blueprints_buildings/BP_farm_01.BP_farm_01_C|Getfield_location_location _asbp_farm_01))))

(event Custom|go%20to%20work
  (Rendering|Components|TextRender|SetText (Variables|Default|Getstatus_OBJECTIVE) (Utilities|Text|ToText(String) (Variables|Default|Getgotowork_text)))
  ;[0.15 0.15 0.15 0.5] on the field
  (AI|Navigation|SimpleMovetoLocation (AI|GetAIController self) (.RandomLocation (AI|Navigation|GetRandomReachablePointinRadius (Variables|Default|Getmy_work) 6e+02 0 0)) :!label _label)
  (Development|PrintText (Utilities|Text|ToText(Float) (Variables|Default|Getclocktime_var) "HalfToEven"))
  (CallFunction|CheckTime)
  (Utilities|FlowControl|Delay 1.0)
  (if (> (Variables|Default|Getclocktime_var) 2.6e+02)
    (CallFunction|GotoHall)
    (else
      (goto _label))))

(event Custom|go%20to%20hall
  (if (Math|Random|RandomBoolwithWeight 0.6)
    (Rendering|Components|TextRender|SetText (Variables|Default|Getstatus_OBJECTIVE) (Utilities|Text|ToText(String) (Variables|Default|Getgotohall_text)))
    (bind _returnvalue (Actor|GetActorOfClass "/Game/blueprints_buildings/BP_hall_01.BP_hall_01_C"))
    (bind _asbp_hall_01 (Utilities|Casting|CastToBP_hall_01 _returnvalue))
    (Variables|Default|Settable_seat (Transformation|GetWorldLocation (.OutItem (Utilities|Array|Random (Utilities|Array|MakeArray (Variables|/Game/blueprints_buildings/BP_hall_01.BP_hall_01_C|Gettable__01_location _asbp_hall_01) (Variables|/Game/blueprints_buildings/BP_hall_01.BP_hall_01_C|Gettable__02_location _asbp_hall_01) (Variables|/Game/blueprints_buildings/BP_hall_01.BP_hall_01_C|Gettable__03_location _asbp_hall_01))))))
    (AI|Navigation|SimpleMovetoLocation (AI|GetAIController self) (Variables|Default|Gettable_seat))
    (Utilities|FlowControl|Delay 3.0)
    (CallFunction|CheckTime)
    (Development|PrintText (Utilities|Text|ToText(Float) (Variables|Default|Getclocktime_var) "HalfToEven") true true "(R=0.000000,G=1.000000,B=0.191608,A=1.000000)")
    (if (>= (Variables|Default|Getclocktime_var) 2.8e+02)
      (Utilities|FlowControl|Delay (Math|Random|RandomFloatinRange 0.0 2.0))
      (CallFunction|GotoBed))
    (else
      (AI|Navigation|SimpleMovetoLocation (AI|GetAIController self) (Variables|Default|Getmy%20bed))
      (Utilities|FlowControl|Delay 5.0)
      (CallFunction|GotoBed))))

(event Custom|go%20to%20bed
  (Rendering|Components|TextRender|SetText (Variables|Default|Getstatus_OBJECTIVE) (Utilities|Text|ToText(String) (Variables|Default|Getgohome_text)))
  (AI|Navigation|SimpleMovetoLocation (AI|GetAIController self) (Variables|Default|Getmy%20bed))
  (Utilities|FlowControl|Delay 1e+01)
  (CallFunction|CheckTime)
  (Rendering|Components|TextRender|SetText (Variables|Default|Getstatus_OBJECTIVE) (Utilities|Text|ToText(String) (Variables|Default|Getsleep_text)))
  (if (> (Variables|Default|Getclocktime_var) 1.6e+02)
    (Utilities|FlowControl|Delay (Math|Random|RandomFloatinRange 0.0 3.0))
    (CallFunction|GotoWork)
    (else
      (CallFunction|GotoBed))))

(event EventTick
  (params (DeltaSeconds :type Float%20%28single-precision%29))
  (Transformation|SetWorldRotation (Variables|Default|Getstatus_root) (Math|Rotator|MakeRotator 0.0 0.0 (.yaw (Math|Rotator|FindLookatRotation (Transformation|GetWorldLocation (Variables|Collision|GetCapsuleComponent)) (Transformation|GetWorldLocation (Variables|/Script/Engine.Actor|GetRootComponent (Game|GetPlayerCameraManager 0)))))) false false))

(event EventBeginPlay
  (Utilities|FlowControl|Delay 2.0)
  (CallFunction|FindMyStuff)
  (CallFunction|FindLocations)
  (CallFunction|DecisionsbyTime))

(fn ConstructionScript)