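; AI night watchman character that lights every BP_lantern_01 in the level, wanders while working, then switches the lanterns off and returns to bed.
; Self-recalling events form the routine, polling Day_night_cycle's clock to leave the sleep and work phases.
; Lantern rounds repeatedly AIMoveTo the nearest remaining lantern, set overlapped lights and drop them from the list.
; Bed location comes from BP_watch_house_01, and an objective status text yaws toward the player camera.
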(event Custom|at%20work
  (Rendering|Components|TextRender|SetText (Variables|Default|Getstatus_OBJECTIVE) (Utilities|Text|ToText(String) (Variables|Default|Getworking_text)))
  (bind _randomlocation (Class|NavigationSystemV1|GetRandomLocationinNavigableRadius (Math|Vector|MakeVector 0.0 0.0 0.0) 1e+03 0 0))
  (AI|Navigation|SimpleMovetoLocation (AI|GetAIController self) _randomlocation)
  (Utilities|FlowControl|Delay 3.0)
  (CallFunction|CheckTime)
  (if (> (Variables|Default|Getclocktime_var) 1.6e+02)
    (CallFunction|Feierabend)
    (else
      (CallFunction|AtWork))))

(event Custom|find%20my%20stuff
  (bind _returnvalue (Actor|GetActorOfClass "/Game/blueprints_buildings/BP_watch_house_01.BP_watch_house_01_C"))
  (bind _asbp_watch_house_01 (Utilities|Casting|CastToBP_watch_house_01 _returnvalue))
  (Variables|Default|Setmy%20bed (Variables|/Game/blueprints_buildings/BP_watch_house_01.BP_watch_house_01_C|Getlocation_BED_var _asbp_watch_house_01))
  (Variables|Default|Setmy%20light (Variables|/Game/blueprints_buildings/BP_watch_house_01.BP_watch_house_01_C|Getlocation_LIGHT_var _asbp_watch_house_01))
  (Variables|Default|Setmy%20home (Variables|/Game/blueprints_buildings/BP_watch_house_01.BP_watch_house_01_C|Getlocation_HOME_var _asbp_watch_house_01)))

(event Custom|check%20time
  (bind _returnvalue (Actor|GetActorOfClass "/Game/blueprints_world_mechanics/day_night_cycle.day_night_cycle_C"))
  (bind _asday_night_cycle (Utilities|Casting|CastToday_night_cycle _returnvalue))
  (Variables|Default|Setclocktime_var (Variables|/Game/blueprints_world_mechanics/day_night_cycle.day_night_cycle_C|GetclockTime _asday_night_cycle))
  (Utilities|FlowControl|Delay 1.0))

(event Custom|go%20to%20work
  (Rendering|Components|TextRender|SetText (Variables|Default|Getstatus_OBJECTIVE) (Utilities|Text|ToText(String) (Variables|Default|Getgotowork_text)))
  (bind _outactors (Actor|GetAllActorsOfClass "/Game/blueprints_buildings/BP_lantern_01.BP_lantern_01_C"))
  (bind _output_get (Variables|Default|SetOut%20Actors _outactors))
  (bind _output_get_2 (Variables|Default|Setlanterns_left_num (Utilities|Array|Length _output_get)))
  (Development|PrintString (Utilities|String|ToString(Integer) _output_get_2) true true "(R=0.000000,G=1.000000,B=0.256324,A=1.000000)" 5.0)
  (AI|AIMoveTo self "0, 0, 0" (.ReturnValue (Actor|FindNearestActor (Transformation|GetWorldLocation (Variables|Collision|GetCapsuleComponent)) (Variables|Default|GetOut%20Actors))) 5.0 false :!label _label
    (:OnSuccess
      (for _array_element (Collision|GetOverlappingActors "/Game/blueprints_buildings/BP_lantern_01.BP_lantern_01_C" :!class /Script/Engine.Actor)
        (Rendering|Components|Light|SetIntensity (Variables|/Game/blueprints_buildings/BP_lantern_01.BP_lantern_01_C|Getlantern_light _array_element) 3e+04)
        (Utilities|Array|RemoveItem (Variables|Default|GetOut%20Actors) _array_element)
        (bind _output_get_3 (Variables|Default|Setlanterns_left_num (- (Variables|Default|Getlanterns_left_num) 1)))
        (Development|PrintString (Utilities|String|ToString(Integer) _output_get_3))
        (if (> (Variables|Default|Getlanterns_left_num) 0)
          (Utilities|FlowControl|Delay 0.0)
          (goto _label)
          (else
            (CallFunction|AtWork)))))
    (:OnFail
      (Development|PrintText "failed" true true "(R=1.000000,G=0.000000,B=0.044178,A=1.000000)" 5.0)
      (CallFunction|AtWork))))

(event Custom|go%20to%20bed
  (AI|Navigation|SimpleMovetoLocation (AI|GetAIController self) (Variables|Default|Getmy%20bed))
  (Utilities|FlowControl|Delay 1.0)
  (Rendering|Components|TextRender|SetText (Variables|Default|Getstatus_OBJECTIVE) (Utilities|Text|ToText(String) (Variables|Default|Getsleeping_text)))
  (CallFunction|CheckTime)
  (if (> (Variables|Default|Getclocktime_var) 3e+02)
    (CallFunction|GotoWork)
    (else
      (CallFunction|GotoBed))))

(event Custom|feierabend
  (Rendering|Components|TextRender|SetText (Variables|Default|Getstatus_OBJECTIVE) (Utilities|Text|ToText(String) (Variables|Default|Getgotowork_text)))
  (bind _outactors (Actor|GetAllActorsOfClass "/Game/blueprints_buildings/BP_lantern_01.BP_lantern_01_C"))
  (bind _output_get (Variables|Default|SetOut%20Actors _outactors))
  (bind _output_get_2 (Variables|Default|Setlanterns_left_num (Utilities|Array|Length _output_get)))
  (Development|PrintString (Utilities|String|ToString(Integer) _output_get_2) true true "(R=0.000000,G=1.000000,B=0.256324,A=1.000000)" 5.0)
  (AI|AIMoveTo self "0, 0, 0" (.ReturnValue (Actor|FindNearestActor (Transformation|GetWorldLocation (Variables|Collision|GetCapsuleComponent)) (Variables|Default|GetOut%20Actors))) 5.0 false :!label _label
    (:OnSuccess
      (for _array_element (Collision|GetOverlappingActors "/Game/blueprints_buildings/BP_lantern_01.BP_lantern_01_C" :!class /Script/Engine.Actor)
        (Rendering|Components|Light|SetIntensity (Variables|/Game/blueprints_buildings/BP_lantern_01.BP_lantern_01_C|Getlantern_light _array_element) 0.0)
        (Utilities|Array|RemoveItem (Variables|Default|GetOut%20Actors) _array_element)
        (bind _output_get_3 (Variables|Default|Setlanterns_left_num (- (Variables|Default|Getlanterns_left_num) 1)))
        (Development|PrintString (Utilities|String|ToString(Integer) _output_get_3))
        (if (> (Variables|Default|Getlanterns_left_num) 0)
          (Utilities|FlowControl|Delay 0.0)
          (goto _label)
          (else
            (CallFunction|GotoBed)))))
    (:OnFail
      (Development|PrintText "failed" true true "(R=1.000000,G=0.000000,B=0.044178,A=1.000000)" 5.0)
      (CallFunction|AtWork))))

(event EventTick
  (params (DeltaSeconds :type Float%20%28single-precision%29))
  (Transformation|SetWorldRotation (Variables|Default|Getstatus_root) (Math|Rotator|MakeRotator 0.0 0.0 (.yaw (Math|Rotator|FindLookatRotation (Transformation|GetWorldLocation (Variables|Collision|GetCapsuleComponent)) (Transformation|GetWorldLocation (Variables|/Script/Engine.Actor|GetRootComponent (Game|GetPlayerCameraManager 0)))))) false false))

(event EventBeginPlay
  (Utilities|FlowControl|Delay 2.0)
  (CallFunction|FindMyStuff)
  (CallFunction|GotoBed))

(fn ConstructionScript)