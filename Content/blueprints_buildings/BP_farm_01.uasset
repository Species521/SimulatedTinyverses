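; BP_farm_01 is a farm building that tells farmer actors where its field is.
; On BeginPlay it stores the world location of its FieldLocation component, then finds every BP_farmer_01 in the level and writes that location into its LocationFieldFarmer.
; The push is one-time and global, with no matching of farmers to a particular farm.
; An unconnected debug print of the location remains in the graph.
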(event EventBeginPlay
  (Variables|Default|Setfield_location_location (Transformation|GetWorldLocation (Variables|Default|Getfield_location)))
  (bind _outactors (Actor|GetAllActorsOfClass "/Game/blueprints_buildings/BP_farmer_01.BP_farmer_01_C"))
  (for _array_element _outactors
    (bind _asbp_farmer_01 (Utilities|Casting|CastToBP_farmer_01 _array_element))
    (Variables|/Game/blueprints_buildings/BP_farmer_01.BP_farmer_01_C|Setlocation_field_farmer _asbp_farmer_01 (Transformation|GetWorldLocation (Variables|Default|Getfield_location)))))

(fn ConstructionScript)