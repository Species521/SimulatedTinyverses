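; Watch house building that spawns a resident farmer AI at its spawn point on BeginPlay and caches its bed, light and home locations.
; On any actor overlap it calls LightsOnoff, then passes BP_farmer_01 actors the light location and state and triggers their TakingCareOfTheLight.
; Point light intensity switching and the home-location handoff to the farmer are left disconnected, and the lightson/off event is empty.
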(event Custom|lights%20on/off)

(event EventBeginPlay
  (Variables|Default|Setlocation_BED_var (Transformation|GetWorldLocation (Variables|Default|Getlocation_BED)))
  (Variables|Default|Setlocation_LIGHT_var (Transformation|GetWorldLocation (Variables|Default|Getlocation_LIGHT)))
  (Variables|Default|Setlocation_HOME_var (Transformation|GetWorldLocation (Variables|Default|Getlocation_HOME)))
  ;[0.15 0.15 0.15 0.5] create resident
  (AI|SpawnAIFromClass "/Game/blueprints_characters/BP_AI_farmer_01.BP_AI_farmer_01_C" 0 (Transformation|GetWorldLocation (Variables|Default|Getlocation_SPAWN)) "0, 0, 0" false 0))

(event Collision|EventActorBeginOverlap
  (params (OtherActor :type Actor%20Object%20Reference))
  (CallFunction|LightsOn/off)
  ;[0.15 0.15 0.15 0.5] light_check
  (bind _asbp_farmer_01 (Utilities|Casting|CastToBP_farmer_01 OtherActor))
  (Variables|/Game/blueprints_buildings/BP_farmer_01.BP_farmer_01_C|Setlocation_light_farmer _asbp_farmer_01 (Transformation|GetWorldLocation (Variables|Default|Getlocation_LIGHT)))
  (Variables|/Game/blueprints_buildings/BP_farmer_01.BP_farmer_01_C|Setlight_state_farmer _asbp_farmer_01 (Variables|Default|Getlight_state))
  (Default|TakingCareOftheLight _asbp_farmer_01))

(fn ConstructionScript)