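; Farmer NPC Blueprint that moves the character between bed, field and hall seating according to a farmer time value.
; The gotobed event prints the time, sends the AI controller to bed early, to the field in the middle window, or randomly to hall or bed late.
; It re-calls itself after a short delay as a polling loop, with a longer pause after each random late-period choice.
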(event Custom|go%20to%20bed
  (Development|PrintText (Utilities|Text|ToText(Float) (Variables|Default|Gettime_farmer) "HalfToEven"))
  (if (> (Variables|Default|Gettime_farmer) 1.8e+02)
    (if (> (Variables|Default|Gettime_farmer) 2.7e+02)
      (if (Math|Random|RandomBool)
        (AI|Navigation|SimpleMovetoLocation (AI|GetAIController self) (Variables|Default|Gethall_seating))
        (Utilities|FlowControl|Delay 5.0)
        (else
          (AI|Navigation|SimpleMovetoLocation (AI|GetAIController self) (Variables|Default|Getlocation_bed_farmer))
          (Utilities|FlowControl|Delay 5.0)))
      (else
        (AI|Navigation|SimpleMovetoLocation (AI|GetAIController self) (Variables|Default|Getfield_location_farmer))))
    (else
      (AI|Navigation|SimpleMovetoLocation (AI|GetAIController self) (Variables|Default|Getlocation_bed_farmer))))
  (Utilities|FlowControl|Delay 0.1)
  (CallFunction|GotoBed))

(fn ConstructionScript)