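; Farmer house building Blueprint that spawns its resident farmer NPC when play begins.
; On BeginPlay it spawns a BP_farmer_01 AI at the LocationSPAWN component.
; It passes the farmer the bed and front-of-house world locations from its marker components, then calls GoToBed on it.
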(event EventBeginPlay
  (bind _returnvalue (AI|SpawnAIFromClass "/Game/blueprints_buildings/BP_farmer_01.BP_farmer_01_C" 0 (Transformation|GetWorldLocation (Variables|Default|Getlocation_SPAWN)) "0, 0, 0" false 0))
  (bind _asbp_farmer_01 (Utilities|Casting|CastToBP_farmer_01 _returnvalue))
  (Variables|/Game/blueprints_buildings/BP_farmer_01.BP_farmer_01_C|Setlocation_bed_farmer _asbp_farmer_01 (Transformation|GetWorldLocation (Variables|Default|Getlocation_BED)))
  (Variables|/Game/blueprints_buildings/BP_farmer_01.BP_farmer_01_C|Setlocation_front_farmer _asbp_farmer_01 (Transformation|GetWorldLocation (Variables|Default|Getlocation_SPAWN)))
  (Default|GotoBed _asbp_farmer_01))

(fn ConstructionScript)