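; BP_hall_01 is a hall building that hands out table seating to farmers and puts the bar keeper to work.
; On BeginPlay it caches the bar's world location and gives every BP_farmer_01 a random one of three table locations as HallSeating, repeating the assignment once per table.
; When a BP_AI_keeper_01 overlaps the bar collider, it calls that keeper's AtWork.
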(event OnComponentBeginOverlap(bar_collider)
  (params (OverlappedComponent :type Primitive%20Component%20Object%20Reference) (OtherActor :type Actor%20Object%20Reference) (OtherComp :type Primitive%20Component%20Object%20Reference) (OtherBodyIndex :type Integer) (bFromSweep :type Boolean) (SweepResult :type Hit%20Result%20Structure%20%28by%20ref%29))
  (bind _asbp_ai_keeper_01 (Utilities|Casting|CastToBP_AI_keeper_01 OtherActor))
  (Default|AtWork _asbp_ai_keeper_01))

(event EventBeginPlay
  (bind _table__03_location (Variables|Default|Gettable__03_location))
  (bind _table__02_location (Variables|Default|Gettable__02_location))
  (bind _table__01_location (Variables|Default|Gettable__01_location))
  (bind _returnvalue (Transformation|GetWorldLocation _table__03_location))
  (bind _returnvalue_2 (Transformation|GetWorldLocation _table__01_location))
  (bind _returnvalue_3 (Transformation|GetWorldLocation _table__02_location))
  (bind _array (Utilities|Array|MakeArray _returnvalue_2 _returnvalue_3 _returnvalue))
  (Variables|Default|Setbar_location_location (Transformation|GetWorldLocation (Variables|Default|Getbar_location)))
  (Utilities|Array|Shuffle _array)
  (for _array_element _array
    (bind _outactors (Actor|GetAllActorsOfClass "/Game/blueprints_buildings/BP_farmer_01.BP_farmer_01_C"))
    (for _array_element_2 _outactors
      (bind _asbp_farmer_01 (Utilities|Casting|CastToBP_farmer_01 _array_element_2))
      (Variables|/Game/blueprints_buildings/BP_farmer_01.BP_farmer_01_C|Sethall_seating _asbp_farmer_01 (.OutItem (Utilities|Array|Random _array))))))

(fn ConstructionScript)